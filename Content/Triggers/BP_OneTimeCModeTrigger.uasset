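; BP_OneTimeCModeTrigger is a trigger actor that temporarily applies a one-time camera mode when the player pawn overlaps it.
; On overlap it casts the player camera manager to PlayerCameraManagerACS and applies the configured OneTimeCameraMode.
; It then waits for that mode's EffectDuration, falling back to a fixed delay if the mode is invalid, and removes the mode.
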(event `self.ReceiveActorBeginOverlap`
  (params (OtherActor :type "Actor Object Reference"))
  (bind _one_time_camera_mode (`self.One Time Camera Mode`))
  (bind _one_time_camera_mode_2 (`self.One Time Camera Mode`))
  (if (== OtherActor (`GameplayStatics.GetPlayerPawn` 0))
    (bind _asplayer_camera_manager_acs (cast `PlayerCameraManagerACS` (`GameplayStatics.GetPlayerCameraManager` 0)))
    (`PlayerCameraManagerACS.ApplyOneTimeCameraMode` _asplayer_camera_manager_acs _one_time_camera_mode_2)
    (`KismetSystemLibrary.Delay` (`KismetMathLibrary.SelectFloat` (`OneTimeCameraMode.EffectDuration` _one_time_camera_mode) 2.0 (`KismetSystemLibrary.IsValid` _one_time_camera_mode)))
    (`PlayerCameraManagerACS.RemoveOneTimeCameraMode` _asplayer_camera_manager_acs _one_time_camera_mode_2)))

(fn `UserConstructionScript`)